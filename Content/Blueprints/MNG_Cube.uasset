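; MNG_Cube is a manager Blueprint that spawns a random prop actor and assigns it to the ControllerProp player controller as its MyBasePawn.
; On BeginPlay it binds a spawn event to a dispatcher, caches the first player controller cast to ControllerProp, and spawns the first prop.
; Each dispatcher broadcast runs SpawnYU again, picking a random class from an array and spawning it at a stored transform.
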(event `Spawn_PRPSSS`
  (`self.SpawnYU`))

(event `self.ReceiveBeginPlay`
  (add `self.Event_Porpsss` (delegate `Spawn_PRPSSS`))
  (bind _ascontroller_prop (cast `/Game/Blueprints/ControllerProp` (`GameplayStatics.GetPlayerController` 0)))
  (set `self.As Controller Prop` _ascontroller_prop)
  (`self.SpawnYU`))

(fn `SpawnYU`
  (bind _returnvalue (`|SpawnActorFromClass` (`KismetArrayLibrary.Array_Random` (`self.BasePROPSSSS`)) (`self.Spawn Transform`) "Undefined" "MultiplyWithRoot" null null))
  (set `/Game/Blueprints/ControllerProp.MyBasePawn` _returnvalue (`self.As Controller Prop`)))

(fn `UserConstructionScript`)