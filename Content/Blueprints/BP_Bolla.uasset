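; BP_Bolla is the bubble of a spirit level, driven by the tilt of a BP_Livella actor.
; It finds and stores the BP_Livella actor on BeginPlay.
; Each Tick it sets its root's roll to the level's roll offset by 90 degrees.
; It also slides the Bubble between RightPos and LeftPos by an unclamped lerp, mapping level roll from 60 to 120 degrees.
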(event `self.ReceiveBeginPlay`
  (bind _returnvalue (`GameplayStatics.GetActorOfClass` "/Game/Blueprints/BP_Livella.BP_Livella_C"))
  (set `self.Livella` _returnvalue))

(event `self.ReceiveTick`
  (params (DeltaSeconds :type "Float (single-precision)"))
  (bind _returnvalue_roll (`KismetMathLibrary.BreakRotator` (`self.K2_GetActorRotation` (`self.Livella`))))
  (bind _returnvalue_roll_2 (`KismetMathLibrary.BreakRotator` (`self.K2_GetActorRotation` (`self.Livella`))))
  (`SceneComponent.K2_SetWorldRotation` (`self.DefaultSceneRoot`) (`KismetMathLibrary.MakeRotator` (- _returnvalue_roll 90.0)) false false)
  (`SceneComponent.K2_SetWorldLocation` (`self.Bubble`) (`KismetMathLibrary.VLerp` (`SceneComponent.K2_GetComponentLocation` (`self.Right pos`)) (`SceneComponent.K2_GetComponentLocation` (`self.Left pos`)) (/ (- _returnvalue_roll_2 60.0) 60.0)) false false))

(fn `UserConstructionScript`)