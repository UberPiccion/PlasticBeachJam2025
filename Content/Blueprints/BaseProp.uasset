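; BaseProp is a falling prop actor that can be nudged sideways and scores points when it first hits something.
; Until that hit, Tick pulls the Cube down with a constant acceleration, while MoveLeft and MoveRight offset it along Y by Speed; MoveDown is empty.
; A DoOnce on the hit enables gravity, tells GM_Bubble to spawn a prop and adds this prop's Score.
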(event `self.Cube.OnComponentHit`
  (params (HitComponent :type "PrimitiveComponent Object Reference") (OtherActor :type "Actor Object Reference") (OtherComp :type "PrimitiveComponent Object Reference") (NormalImpulse :type "Vector Structure") (Hit :type "HitResult Structure (by ref)"))
  (`/Engine/EditorBlueprintResources/StandardMacros.DoOnce` false
    (:`Completed`
      (bind _asgm_bubble (cast `/Game/Blueprints/GM_Bubble` (`GameplayStatics.GetGameMode`)))
      (`/Game/Blueprints/GM_Bubble.EventSpawnProp_Event` _asgm_bubble)
      (`PrimitiveComponent.SetEnableGravity` (`self.Cube`) true)
      (set `self.HasGravity` true)
      (bind _asgm_bubble_2 (cast `/Game/Blueprints/GM_Bubble` (`GameplayStatics.GetGameMode`)))
      (`/Game/Blueprints/GM_Bubble.AddScore` _asgm_bubble_2 (`self.Score`)))))

(event `self.ReceiveTick`
  (params (DeltaSeconds :type "Float (single-precision)"))
  ;[1 1 1] Cerchiamo un metodo alternativo
  (if (not (`self.HasGravity`))
    (`PrimitiveComponent.AddForce` (`self.Cube`) (0.0 0.0 -100.0) "None" true)))

(event `Move Right`
  (`self.K2_SetActorLocation` (+ (`self.K2_GetActorLocation`) (`KismetMathLibrary.MakeVector` 0.0 (* (`self.Speed`) 1.0)))))

(event `Move Left`
  (`self.K2_SetActorLocation` (+ (`self.K2_GetActorLocation`) (`KismetMathLibrary.MakeVector` 0.0 (* (`self.Speed`) -1.0)))))

(event `Move Down`)

(fn `UserConstructionScript`)