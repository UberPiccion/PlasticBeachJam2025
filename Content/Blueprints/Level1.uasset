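; Level1 Blueprint holds session state (player name, score and level) and handles saving and background music.
; StartOST spawns a quiet 2D track that persists across level transitions, only when no valid one exists.
; Small functions set the level, add to the score and reset all three values.
; SaveData appends the current record to the SaveGameBubble in a fixed slot, creating the save object if loading fails.
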(event `StartOST`
  (`self.OST `
    (:`then`)
    (:`else`
      (bind _returnvalue (`GameplayStatics.SpawnSound2D` "/Game/Sounds/SFX_Background.SFX_Background" 0.04 1.0 0.0 null true))
      (set `self.OST ` _returnvalue))))

(fn `Change Level`
  (params (NewLevel :type Integer :default 1))
  (set `self.Level` NewLevel))

(fn `Change Score`
  (params (`Score To Add` :type Integer))
  (set `self.Score` (+ `Score To Add` (`self.Score`))))

(fn `ResetDatas`
  (set `self.Level` 0)
  (set `self.Score` 0)
  (set `self.Giulio'sName` ""))

(fn `SaveData`
  (bind _returnvalue (`GameplayStatics.LoadGameFromSlot` "SaveSlot1"))
  (`/Engine/EditorBlueprintResources/StandardMacros.IsValid` _returnvalue
    (:`Is Valid`
      (bind _assave_game_bubble (cast `/Game/Blueprints/SaveGameBubble` _returnvalue))
      (`KismetArrayLibrary.Array_Add` (`/Game/Blueprints/SaveGameBubble.Datas` _assave_game_bubble) (make `/Game/Blueprints/SaveDataSNM` (`self.Giulio'sName`) (`self.Score`) (`self.Level`)))
      (`GameplayStatics.SaveGameToSlot` _assave_game_bubble "SaveSlot1"))
    (:`Is Not Valid`
      (bind _returnvalue_2 (`GameplayStatics.CreateSaveGameObject` "/Game/Blueprints/SaveGameBubble.SaveGameBubble_C"))
      (`KismetArrayLibrary.Array_Add` (`/Game/Blueprints/SaveGameBubble.Datas` _returnvalue_2) (make `/Game/Blueprints/SaveDataSNM` (`self.Giulio'sName`) (`self.Score`) (`self.Level`)))
      (`GameplayStatics.SaveGameToSlot` _returnvalue_2 "SaveSlot1"))))