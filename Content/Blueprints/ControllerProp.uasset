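; ControllerProp is a player controller that handles left/right movement input and the pause menu.
; On BeginPlay it adds the moving and pause input mapping contexts and creates a hidden UI_Pause widget.
; MoveLeft and MoveRight forward to MyBasePawn while triggered or ongoing; Drop has no logic.
; Pause toggles game pause and the menu, removing the movement context while paused so only pause input stays mapped.
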(event `self.ReceiveBeginPlay`
  (bind _returnvalue (pcsubsystem `EnhancedInputLocalPlayerSubsystem` self))
  (`EnhancedInputSubsystemInterface.AddMappingContext` _returnvalue "/Game/Input/IContextMoving.IContextMoving" 0 (struct))
  (`EnhancedInputSubsystemInterface.AddMappingContext` _returnvalue "/Game/Input/IContextPause.IContextPause" 0 (struct))
  (bind _returnvalue_2 (`|CreateWidget` "/Game/Ui/UI_Pause.UI_Pause_C"))
  (bind _output_get (set `self.PauseUI` _returnvalue_2))
  (`UserWidget.AddToViewport` _output_get 0)
  (`Widget.SetVisibility` _output_get "Hidden"))

(event `EnhancedInput|/Game/Input/MoveLeft`
  (params (ActionValue :type Boolean) (ElapsedSeconds :type "Float (double-precision)") (TriggeredSeconds :type "Float (double-precision)") (InputAction :type "InputAction Object Reference" :default "/Game/Input/MoveLeft.MoveLeft"))
  (:`Triggered`
    (bind _mybasepawn (`self.MyBasePawn` :!label _label)
      (:`then`
        (`/Game/Blueprints/Objects/BaseProp.Move Left` _mybasepawn))
      (:`else`)))
  (:`Ongoing`
    (goto _label)))

(event `EnhancedInput|/Game/Input/MoveRight`
  (params (ActionValue :type Boolean) (ElapsedSeconds :type "Float (double-precision)") (TriggeredSeconds :type "Float (double-precision)") (InputAction :type "InputAction Object Reference" :default "/Game/Input/MoveRight.MoveRight"))
  (:`Triggered`
    (bind _mybasepawn (`self.MyBasePawn` :!label _label_2)
      (:`then`
        (`/Game/Blueprints/Objects/BaseProp.Move Right` _mybasepawn))
      (:`else`)))
  (:`Ongoing`
    (goto _label_2)))

(event `EnhancedInput|/Game/Input/Drop`
  (params (ActionValue :type Boolean) (ElapsedSeconds :type "Float (double-precision)") (TriggeredSeconds :type "Float (double-precision)") (InputAction :type "InputAction Object Reference" :default "/Game/Input/Drop.Drop")))

(event `EnhancedInput|/Game/Input/Pause`
  (params (ActionValue :type Boolean) (ElapsedSeconds :type "Float (double-precision)") (TriggeredSeconds :type "Float (double-precision)") (InputAction :type "InputAction Object Reference" :default "/Game/Input/Pause.Pause"))
  (bind _returnvalue (pcsubsystem `EnhancedInputLocalPlayerSubsystem` self))
  (:`Triggered`
    (if (`GameplayStatics.IsGamePaused`)
      (`EnhancedInputSubsystemInterface.AddMappingContext` _returnvalue "/Game/Input/IContextMoving.IContextMoving" 0 (struct))
      (`GameplayStatics.SetGamePaused` false)
      (`Widget.SetVisibility` (`self.PauseUI`) "Hidden")
      (else
        (`EnhancedInputSubsystemInterface.RemoveMappingContext` _returnvalue "/Game/Input/IContextMoving.IContextMoving" (struct))
        (`GameplayStatics.SetGamePaused` true)
        (`Widget.SetVisibility` (`self.PauseUI`) "Visible")))))

(fn `UserConstructionScript`)