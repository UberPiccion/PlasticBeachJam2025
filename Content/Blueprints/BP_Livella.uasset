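; BP_Livella is an actor, named after a spirit level, that rates its own tilt as a score multiplier.
; ScoreMultiplier measures how far the actor's roll deviates from 90 degrees and checks it against MaxScoreAngle, then MediumScoreAngle, returning a triple, double or single multiplier.
; The event graph and construction script are empty, so the actor does nothing until that function is called.
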(fn `ScoreMultiplier`
  (returns (Multiplier :type "Float (double-precision)"))
  (bind _returnvalue_roll (`KismetMathLibrary.BreakRotator` (`self.K2_GetActorRotation`)))
  (bind _returnvalue (`KismetMathLibrary.Abs` (- _returnvalue_roll 90.0)))
  (if (<= _returnvalue (`self.MaxScoreAngle`))
    (return 3.0)
    (elif (<= _returnvalue (`self.MediumScoreAngle`))
      (return 2.0)
      (else
        (return 1.0)))))

(fn `UserConstructionScript`)