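; Base prop for a bubble game: a cube that moves sideways along Y and scores when it lands on something other than a DestroyProps actor.
; Until gravity is enabled, Tick applies a Z acceleration.
; Overlap and hit events, gated by DoOnce, add multiplied score through GM_Bubble or treat DestroyProps contact as a loss.
; Either outcome turns gravity on and asks the game mode to spawn the next prop.
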(event `self.Cube.OnComponentBeginOverlap`
  (params (OverlappedComponent :type "PrimitiveComponent Object Reference") (OtherActor :type "Actor Object Reference") (OtherComp :type "PrimitiveComponent Object Reference") (OtherBodyIndex :type Integer) (bFromSweep :type Boolean) (SweepResult :type "HitResult Structure (by ref)"))
  (`/Engine/EditorBlueprintResources/StandardMacros.DoOnce` (`self.DoOnce`)
    (:`Completed`
      (cast `/Game/Blueprints/DestroyProps` OtherActor
        (:`then`
          (`GameplayStatics.PlaySound2D` (`self.DeathSound`) 1.0 1.0 0.0 null null)
          (`self.SpawnNew`))
        (:`CastFailed`
          (`GameplayStatics.PlaySound2D` (`self.HitSound`) 1.0 1.0 0.0 null null :!label _label)
          (bind _asgm_bubble (cast `/Game/Blueprints/GM_Bubble` (`GameplayStatics.GetGameMode`)))
          (`/Game/Blueprints/GM_Bubble.AddScore` _asgm_bubble (`KismetMathLibrary.FTrunc` (* (`self.Score`) (`self.ScoreMultipier`))))
          (`self.SpawnNew`)))
      (set `self.DoOnce` true :!label _label_2))))

(event `self.Cube.OnComponentHit`
  (params (HitComponent :type "PrimitiveComponent Object Reference") (OtherActor :type "Actor Object Reference") (OtherComp :type "PrimitiveComponent Object Reference") (NormalImpulse :type "Vector Structure") (Hit :type "HitResult Structure (by ref)"))
  (`/Engine/EditorBlueprintResources/StandardMacros.DoOnce` (`self.DoOnce`)
    (:`Completed`
      (cast `/Game/Blueprints/DestroyProps` OtherActor
        (:`then`
          (`self.SpawnNew`)
          (goto _label_2))
        (:`CastFailed`
          (goto _label))))))

(event `self.ReceiveTick`
  (params (DeltaSeconds :type "Float (single-precision)"))
  ;[1 1 1] Cerchiamo un metodo alternativo
  (if (not (`self.HasGravity`))
    (`PrimitiveComponent.AddForce` (`self.Cube`) (`KismetMathLibrary.MakeVector` 0.0 0.0 (`self.Force Z`)) "None" true)))

(event `Move Right`
  (`self.K2_SetActorLocation` (+ (`self.K2_GetActorLocation`) (`KismetMathLibrary.MakeVector` 0.0 (* (`self.Speed`) 1.0)))))

(event `Move Left`
  (`self.K2_SetActorLocation` (+ (`self.K2_GetActorLocation`) (`KismetMathLibrary.MakeVector` 0.0 (* (`self.Speed`) -1.0)))))

(event `Move Down`)

(fn `SpawnNew`
  (`PrimitiveComponent.SetEnableGravity` (`self.Cube`) true)
  (set `self.HasGravity` true)
  (bind _asgm_bubble (cast `/Game/Blueprints/GM_Bubble` (`GameplayStatics.GetGameMode`)))
  (`/Game/Blueprints/GM_Bubble.EventSpawnProp` _asgm_bubble))

(fn `UserConstructionScript`)