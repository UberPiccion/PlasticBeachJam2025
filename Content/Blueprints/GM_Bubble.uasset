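; GM_Bubble is the game mode that runs a level's prop spawning, lives, score and progression.
; On BeginPlay it creates the game UI and reads the score target from DT_LevelDataGiulio using the Level1 game instance's level index.
; A spawn event creates random props and hands them to ControllerProp.
; Reaching the target passes score times BP_Livella's truncated multiplier to Level1 and opens the next level; losing all lives opens MainMenu.
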(event `EventSpawnProp_Event`
  (`self.SpawnYU`))

(event `self.ReceiveBeginPlay`
  (bind _ascontroller_prop (cast `/Game/Blueprints/ControllerProp` (`GameplayStatics.GetPlayerController` 0)))
  (set `self.As Controller Prop` _ascontroller_prop)
  (add `self.EventSpawnProp` (delegate `EventSpawnProp_Event`))
  (`self.EventSpawnProp_Event`)
  (bind _returnvalue (`|CreateWidget` "/Game/Ui/Ui_Game.Ui_Game_C" (`GameplayStatics.GetPlayerController` 0)))
  (`UserWidget.AddToViewport` _returnvalue 0)
  (bind _returnvalue_2 (`GameplayStatics.GetActorOfClass` "/Game/Blueprints/BP_Livella.BP_Livella_C"))
  (set `self.Livella` _returnvalue_2)
  (set `self.Curr Lifes` (`self.Max Lifes`))
  (bind _aslevel_1 (cast `/Game/Blueprints/Level1` (`GameplayStatics.GetGameInstance`)))
  (bind _outrownames (`DataTableFunctionLibrary.GetDataTableRowNames` "/Game/Blueprints/DT_LevelDataGiulio.DT_LevelDataGiulio"))
  (bind _returnvalue_3 (`|GetDataTableRow` "/Game/Blueprints/DT_LevelDataGiulio.DT_LevelDataGiulio" (`|GetArrayItem` _outrownames (`/Game/Blueprints/Level1.Level` _aslevel_1)))
    (:`then`
      (set `self.MaxScore` (break `/Game/Blueprints/LevelScoreSNM` _returnvalue_3)))))

(fn `Add Lifes`
  (params (LifesToIncrement :type Integer :default 1))
  (returns (CurrLifes :type Integer))
  (bind _max_lifes (`self.Max Lifes`))
  (bind _returnvalue (+ LifesToIncrement (`self.Curr Lifes`)))
  (if (<= _returnvalue _max_lifes)
    (set `self.Curr Lifes` _returnvalue)
    (else
      (set `self.Curr Lifes` _max_lifes)))
  (return (`self.Curr Lifes`)))

(fn `AddScore`
  (params (ScoreToAdd :type Integer))
  (returns (Score :type Integer))
  (bind _output_get (set `self.Score` (+ (`self.Score`) ScoreToAdd)))
  (`self.EventUpdateScore`)
  (if (>= _output_get (`self.MaxScore`))
    (bind _aslevel_1 (cast `/Game/Blueprints/Level1` (`GameplayStatics.GetGameInstance`)))
    (`/Game/Blueprints/Level1.Change Score` _aslevel_1 (* (`self.Score`) (`KismetMathLibrary.FTrunc` (`/Game/Blueprints/BP_Livella.ScoreMultiplier` (`self.Livella`)))))
    (bind _outrownames (`DataTableFunctionLibrary.GetDataTableRowNames` "/Game/Blueprints/DT_LevelDataGiulio.DT_LevelDataGiulio"))
    (bind _level (`/Game/Blueprints/Level1.Level` _aslevel_1))
    (bind _returnvalue (`|GetDataTableRow` "/Game/Blueprints/DT_LevelDataGiulio.DT_LevelDataGiulio" (`|GetArrayItem` _outrownames _level))
      (:`then`
        (set `/Game/Blueprints/Level1.Level` (+ _level 1) _aslevel_1)
        (`GameplayStatics.OpenLevel` (`.NextLeve_7_B2B46DE94CD083AE28B793822EF640D9` (break `/Game/Blueprints/LevelScoreSNM` _returnvalue)))))
    (else
      (return _output_get))))

(fn `IncrementTotalLifes`
  (params (LifeToIncrement :type Integer))
  (set `self.Max Lifes` (+ LifeToIncrement (`self.Max Lifes`)))
  (set `self.Curr Lifes` (+ (`local.LifeToIncrement`) (`self.Curr Lifes`))))

(fn `Lose Life`
  (bind _result (`/Engine/EditorBlueprintResources/StandardMacros.DecrementInt` (`self.Curr Lifes`))
    (:`  `
      (`self.EventLoseLife`)
      (if (<= _result 0)
        (`GameplayStatics.OpenLevel` "MainMenu")))))

(fn `LoseScore`
  (params (ScoreToSubtract :type Integer))
  (returns (Score :type Integer))
  (bind _output_get (set `self.Score` (- (`self.Score`) ScoreToSubtract)))
  (`self.EventUpdateScore`)
  (return _output_get))

(fn `SpawnYU`
  (bind _returnvalue (`|SpawnActorFromClass` (`KismetArrayLibrary.Array_Random` (`self.BasePropToSpawn`)) (`self.Spawn Transform`) "AdjustIfPossibleButAlwaysSpawn" "MultiplyWithRoot" null null))
  (set `/Game/Blueprints/ControllerProp.MyBasePawn` _returnvalue (`self.As Controller Prop`)))

(fn `UserConstructionScript`)