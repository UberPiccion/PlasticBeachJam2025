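; DestroyProps is an actor with a Box trigger that penalises the player when a prop touches it.
; It caches the GM_Bubble game mode on BeginPlay.
; When a BaseProp overlaps the box, the game mode loses the prop's score times its multiplier, truncated, plus a life, and the prop is destroyed.
; A leftover score-update call sits unconnected and never runs.
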(event `self.ReceiveBeginPlay`
  (bind _asgm_bubble (cast `/Game/Blueprints/GM_Bubble` (`GameplayStatics.GetGameMode`)))
  (set `self.As GM Bubble` _asgm_bubble))

(event `self.Box.OnComponentBeginOverlap`
  (params (OverlappedComponent :type "PrimitiveComponent Object Reference") (OtherActor :type "Actor Object Reference") (OtherComp :type "PrimitiveComponent Object Reference") (OtherBodyIndex :type Integer) (bFromSweep :type Boolean) (SweepResult :type "HitResult Structure (by ref)"))
  (bind _as_gm_bubble (`self.As GM Bubble`))
  (bind _asbase_prop (cast `/Game/Blueprints/Objects/BaseProp` OtherActor))
  (`/Game/Blueprints/GM_Bubble.LoseScore` _as_gm_bubble (`KismetMathLibrary.FTrunc` (* (`/Game/Blueprints/Objects/BaseProp.Score` _asbase_prop) (`/Game/Blueprints/Objects/BaseProp.ScoreMultipier` _asbase_prop))))
  (`/Game/Blueprints/GM_Bubble.Lose Life` _as_gm_bubble)
  (`self.K2_DestroyActor` _asbase_prop))

(fn `UserConstructionScript`)